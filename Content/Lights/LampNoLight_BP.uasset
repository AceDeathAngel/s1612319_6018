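; Lamp Blueprint, apparently for traffic lights, that shows on, off and flashing states purely through mesh materials.
; SwitchLampState plays or reverses the LightAnimation timeline, scaling its rate by switch or cycle time, and ping-pongs it while flashing.
; The timeline drives the material's LightSwitch parameter, and the construction script sets its Colour.
; Leftover light intensity and colour nodes are disconnected.
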(event Custom|Switch%20Lamp%20State
  (params (State :type lampState%20Enum :default "NewEnumerator0"))
  (bind _lightanimation (Variables|Default|GetLightAnimation))
  (bind _lightanimation_2 (Variables|Default|GetLightAnimation))
  (bind _lightanimation_3 (Variables|Default|GetLightAnimation))
  (switch Utilities|FlowControl|Switch|SwitchonlampState State
    (:NewEnumerator0
      ;[1 1 1] Swiches the Light on
      (Variables|Default|SetFlashing? false)
      (Components|Timeline|SetPlayRate _lightanimation_3 (/ 1.0 (Variables|Default|GetOnOffTime)))
      (Audio|Components|Audio|Play _lightanimation_3))
    (:NewEnumerator1
      ;[1 1 1] Swiches Light off
      (Variables|Default|SetFlashing? false)
      (Components|Timeline|SetPlayRate _lightanimation (/ 1.0 (Variables|Default|GetOnOffTime)))
      (Utilities|String|Reverse _lightanimation))
    (:NewEnumerator2
      ;[1 1 1] sets flashing light
      (Variables|Default|SetFlashing? true)
      (Components|Timeline|SetPlayRate _lightanimation_2 (/ 2.0 (Variables|Default|GetCycleTime)))
      (Audio|Components|Audio|Play _lightanimation_2))))

(fn ConstructionScript
  ;[1 1 1] Sets the lamp and point light colour on trafic light
  (Rendering|Material|SetVectorParameterValueonMaterials (Variables|Default|GetLampMesh) "Colour" (Math|Conversions|ToVector(LinearColor) (Variables|Default|GetColour))))