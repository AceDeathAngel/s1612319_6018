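; Pedestrian crossing traffic light that drives child-actor lamps for vehicles and pedestrians, two wait lamps and crossing beepers.
; It rests on green until ButtonPressed is set externally, then a Tick timer runs amber, red and red-amber before returning to green.
; ChangeLightState sets the signal lamps per state and clears request flags.
; Tick mirrors WaitLightOn to the wait lamps and plays the beeps while LightIsRed is true.
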(event Custom|ChangeLightState
  (params (State :type TrafficLightState%20Enum :default "NewEnumerator0"))
  (bind _amber (Variables|Default|GetAmber))
  (bind _green (Variables|Default|GetGreen))
  (bind _redpedestrian (Variables|Default|GetRedPedestrian))
  (bind _greenpedestrian (Variables|Default|GetGreenPedestrian))
  (bind _red (Variables|Default|GetRed))
  ;[1 1 1] determins which lights are on depending on the state
  (bind _output_get (Variables|Default|Setstate State))
  (Variables|Default|SetTimer 0.0)
  (switch Utilities|FlowControl|Switch|SwitchonTrafficLightState _output_get
    (:NewEnumerator0
      (Default|SwitchLampState _red "NewEnumerator0")
      (Default|SwitchLampState _amber "NewEnumerator1")
      (Default|SwitchLampState _green "NewEnumerator1")
      (Default|SwitchLampState _greenpedestrian "NewEnumerator0")
      (Default|SwitchLampState _redpedestrian "NewEnumerator1")
      ;;[1 0 0] send message to Veichel BP
      (Variables|Default|SetLightIsRed true)
      (Variables|Default|SetWaitLightOn false))
    (:NewEnumerator1
      (Default|SwitchLampState _red "NewEnumerator0")
      (Default|SwitchLampState _amber "NewEnumerator0")
      (Default|SwitchLampState _green "NewEnumerator1")
      (Default|SwitchLampState _greenpedestrian "NewEnumerator1")
      (Default|SwitchLampState _redpedestrian "NewEnumerator0"))
    (:NewEnumerator2
      (Default|SwitchLampState _red "NewEnumerator1")
      (Default|SwitchLampState _amber "NewEnumerator0")
      (Default|SwitchLampState _green "NewEnumerator1")
      (Default|SwitchLampState _greenpedestrian "NewEnumerator1")
      (Default|SwitchLampState _redpedestrian "NewEnumerator0"))
    (:NewEnumerator3
      (Default|SwitchLampState _red "NewEnumerator1")
      (Default|SwitchLampState _amber "NewEnumerator1")
      (Default|SwitchLampState _green "NewEnumerator0")
      (Default|SwitchLampState _greenpedestrian "NewEnumerator1")
      (Default|SwitchLampState _redpedestrian "NewEnumerator0")
      (Variables|Default|SetButtonPressed false))))

(event EventBeginPlay
  (bind _aslamp_bp (Utilities|Casting|CastToLamp_BP (Variables|/Script/Engine.ChildActorComponent|GetChildActor (Variables|Default|GetRedLight))))
  (Variables|Default|SetRed _aslamp_bp)
  (bind _aslamp_bp_2 (Utilities|Casting|CastToLamp_BP (Variables|/Script/Engine.ChildActorComponent|GetChildActor (Variables|Default|GetAmberLight))))
  (Variables|Default|SetAmber _aslamp_bp_2)
  (bind _aslamp_bp_3 (Utilities|Casting|CastToLamp_BP (Variables|/Script/Engine.ChildActorComponent|GetChildActor (Variables|Default|GetGreenLight))))
  (Variables|Default|SetGreen _aslamp_bp_3)
  (bind _aslamp_bp_4 (Utilities|Casting|CastToLamp_BP (Variables|/Script/Engine.ChildActorComponent|GetChildActor (Variables|Default|GetGreenLightPedestrian))))
  (Variables|Default|SetGreenPedestrian _aslamp_bp_4)
  (bind _aslamp_bp_5 (Utilities|Casting|CastToLamp_BP (Variables|/Script/Engine.ChildActorComponent|GetChildActor (Variables|Default|GetRedLightPedestrian))))
  (Variables|Default|SetRedPedestrian _aslamp_bp_5)
  (bind _aslamp_no_light_bp (Utilities|Casting|CastToLampNoLight_BP (Variables|/Script/Engine.ChildActorComponent|GetChildActor (Variables|Default|GetWaitLight))))
  (Variables|Default|SetWait _aslamp_no_light_bp)
  (bind _aslamp_no_light_bp_2 (Utilities|Casting|CastToLampNoLight_BP (Variables|/Script/Engine.ChildActorComponent|GetChildActor (Variables|Default|GetWaitLight1))))
  (Variables|Default|SetWait1 _aslamp_no_light_bp_2)
  (CallFunction|ChangeLightState "NewEnumerator3"))

(event EventTick
  (params (DeltaSeconds :type Float%20%28single-precision%29))
  (bind _lightbeep2 (Variables|Default|GetLightBeep2))
  (bind _lightbeep1 (Variables|Default|GetLightBeep1))
  (bind _wait (Variables|Default|GetWait))
  (bind _wait1 (Variables|Default|GetWait1))
  ;[1 1 1] cycles through the states of the lights and checks the timer
  (Utilities|FlowControl|Sequence
    (:then_0
      (if (Variables|Default|GetButtonPressed)
        (Variables|Default|SetTimer (+ DeltaSeconds (Variables|Default|GetTimer)))
        (switch Utilities|FlowControl|Switch|SwitchonTrafficLightState (Variables|Default|Getstate)
          (:NewEnumerator0
            (if (> (Variables|Default|GetTimer) (Variables|Default|GetRedTime))
              (CallFunction|ChangeLightState "NewEnumerator1")))
          (:NewEnumerator1
            (if (> (Variables|Default|GetTimer) (Variables|Default|GetAmberRedTime))
              (CallFunction|ChangeLightState "NewEnumerator3")
              (Variables|Default|SetLightIsRed false)))
          (:NewEnumerator2
            (if (> (Variables|Default|GetTimer) (Variables|Default|GetAmberTime))
              (CallFunction|ChangeLightState "NewEnumerator0")))
          (:NewEnumerator3
            (if (> (Variables|Default|GetTimer) (Variables|Default|GetGreenTime))
              (CallFunction|ChangeLightState "NewEnumerator2"))))))
    (:then_1
      ;;[1 0 0] Wait button light switch
      (if (Variables|Default|GetWaitLightOn)
        (Default|SwitchLampState _wait "NewEnumerator0")
        (else
          (Default|SwitchLampState _wait "NewEnumerator1"))))
    (:then_2
      (if (Variables|Default|GetWaitLightOn)
        (Default|SwitchLampState _wait1 "NewEnumerator0")
        (else
          (Default|SwitchLampState _wait1 "NewEnumerator1"))))
    (:then_3
      ;;[1 0 0] Plays Audio beeding audio when light is red
      (if (Variables|Default|GetLightIsRed)
        (if (not (Variables|Default|GetAudioIsPlaying))
          (Class|FMODAudioComponent|Play _lightbeep1)
          (Class|FMODAudioComponent|Play _lightbeep2)
          (Variables|Default|SetAudioIsPlaying true))
        (else
          (Class|FMODAudioComponent|Stop _lightbeep1)
          (Class|FMODAudioComponent|Stop _lightbeep2)
          (Variables|Default|SetAudioIsPlaying false))))))

(fn ConstructionScript)