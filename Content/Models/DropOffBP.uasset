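; Drop-off point Blueprint that completes the level when the player brings the held ball to it.
; Tick reveals the mesh once, when the referenced PickUpBall reports it has been picked up.
; The first overlap while the ball is held plays FMOD audio, toggles the mesh's visibility and flags WellDoneBP to switch on.
; After a delay it starts a camera fade and immediately opens MenuScene.
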(event Collision|EventActorBeginOverlap
  (params (OtherActor :type Actor%20Object%20Reference))
  ;[1 0 0] Check if the ball is held on colliison switches visability of drop off, plays well doen audio and takes the player back to the main menu.
  (if (Variables|/Game/Interactabls/PickupBall.PickupBall_C|GetBallHeld (Variables|Default|GetPickUpBall))
    (if (not (Variables|Default|GetCylinderTrigered))
      (Variables|Default|SetCylinderTrigered true)
      (Class|FMODAudioComponent|Play (Variables|Default|GetFMODAudio))
      (Rendering|ToggleVisibility (Variables|Debug|GetStaticMeshComponent) false)
      (Variables|/Game/Widgets/RoadCrossWidgets/WellDoneBP.WellDoneBP_C|SetSwitchOnWellDone (Variables|Default|GetWellDoneBP) true)
      (Utilities|FlowControl|Delay 1e+01)
      (CameraFades|StartCameraFade :self (Game|GetPlayerCameraManager 0) :ToAlpha 1.0 :Duration 1.0)
      (Game|OpenLevel(byName) "MenuScene"))))

(event EventTick
  (params (DeltaSeconds :type Float%20%28single-precision%29))
  ;[1 0 0] Check if the ball has been picked and then sets visbility
  (if (not (Variables|Default|GetHasTicked))
    (if (Variables|/Game/Interactabls/PickupBall.PickupBall_C|GetPickedUp (Variables|Default|GetPickUpBall))
      (Rendering|SetVisibility (Variables|Debug|GetStaticMeshComponent) true false)
      (Variables|Default|SetHasTicked true))))

(fn ConstructionScript)